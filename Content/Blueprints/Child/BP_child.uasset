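; BP_child is an AI-driven child actor that watches a target and decides when to scream.
; A looping timer turns its yaw toward the target while one is set.
; While Counter remains positive, a forward-vector dot product detects the target facing away, sets the scream Blackboard flag and spawns a short-lived fire storm, gated by DoOnce.
; BeginPlay seeds the Blackboard with the counter and an exit location; SetCounter decrements the counter.
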(event Custom|StartLookingAt
  (bind _returnvalue (Transformation|GetActorRotation))
  (Utilities|IsValid (Variables|Default|GetTarget%20Actor)
    (:Is%20Valid
      (Transformation|SetActorRotation (Math|Rotator|MakeRotator (.roll _returnvalue) (.pitch _returnvalue) (.yaw (Math|Rotator|FindLookatRotation (Transformation|GetActorLocation) (Transformation|GetActorLocation (Variables|Default|GetTarget%20Actor))))))
      (CallFunction|ShouldScream))))

(event Custom|SetTarget
  (params (Target%20Actor :type Actor%20Object%20Reference))
  (bind _output_get (Variables|Default|SetTarget%20Actor Target%20Actor))
  (Utilities|IsValid _output_get
    (:Is%20Valid
      (if (not (Utilities|Time|IsTimerActivebyHandle (Variables|Default|GetLookAtTH)))
        (bind _returnvalue (Utilities|Time|SetTimerbyEvent (delegate Custom|StartLookingAt) 0.2 true))
        (Variables|Default|SetLookAtTH _returnvalue)))
    (:Is%20Not%20Valid
      (Utilities|Time|ClearandInvalidateTimerbyHandle (Variables|Default|GetLookAtTH))
      (AI|Components|Blackboard|SetValueasBool (AI|GetBlackboard 0) (Variables|Default|GetBBShouldScream) false))))

(event Custom|ShouldScream
  (bind _returnvalue (Transformation|GetActorForwardVector))
  (bind _target_actor (Variables|Default|GetTarget%20Actor))
  (bind _returnvalue_2 (Transformation|GetActorForwardVector _target_actor))
  (bind _returnvalue_3 (Math|Vector|DotProduct _returnvalue _returnvalue_2))
  (bind _returnvalue_4 (> _returnvalue_3 0.7))
  (if (> (Variables|Default|GetCounter) 0)
    (Utilities|IsValid _target_actor
      (:Is%20Valid
        (AI|Components|Blackboard|SetValueasBool (AI|GetBlackboard 0) (Variables|Default|GetBBShouldScream) _returnvalue_4)
        (if _returnvalue_4
          (Utilities|IsValid (Variables|Default|GetStorm)
            (:Is%20Not%20Valid
              (Utilities|FlowControl|DoOnce false :!label _label
                (:Completed
                  (bind _returnvalue_5 (Game|SpawnActorfromClass "/Game/FXVarietyPack/Blueprints/BP_ky_fireStorm.BP_ky_fireStorm_C" (Math|Transform|MakeTransform (Transformation|GetActorLocation) "0, 0, 0" "1,1,1") "AlwaysSpawn" 0 0))
                  (bind _output_get (Variables|Default|SetStorm _returnvalue_5))
                  (Actor|SetLifeSpan _output_get 1.0)))))
          (else
            (goto _label Reset)))))))

(event EventBeginPlay
  (bind _returnvalue (AI|GetBlackboard 0))
  (Class|BlackboardComponent|SetValueasInt _returnvalue (Variables|Default|GetBBCounter) (Variables|Default|GetCounter))
  (AI|Components|Blackboard|SetValueasVector _returnvalue (Variables|Default|GetBBOutLocation) "-1500.000000,2420.000000,610.000000"))

(event EventTick
  (params (DeltaSeconds :type Float%20%28single-precision%29)))

(fn ConstructionScript)

(fn GetCounter
  (return (Variables|Default|GetCounter)))

(fn SetCounter
  (bind _result (Math|Integer|DecrementInt (Variables|Default|GetCounter))
    (:%20%20
      (Variables|Default|SetCounter _result))))